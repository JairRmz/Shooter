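; GS_TDM is a team deathmatch game state that tracks the alive count for Team A and Team B.
; DecreaseTeamNumber lowers the given team's count and, when it reaches zero, shows a WB_WinnerTeam widget announcing the other team as winner.
; Otherwise UpdateWidget writes both counts to the local player character's HUD, which also happens shortly after BeginPlay.
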(event Custom|DecreaseTeamNumber
  (params (Team%20A :type Boolean))
  (if Team%20A
    (bind _result (Math|Integer|DecrementInt (Variables|Default|GetNumberOfTeamA_Alive))
      (:%20%20
        (if (<= _result 0)
          (bind _returnvalue (UserInterface|CreateWidget "/Game/WB_WinnerTeam.WB_WinnerTeam_C"))
          (Rendering|Components|TextRender|SetText (Variables|/Game/WB_WinnerTeam.WB_WinnerTeam_C|GetWinnerText _returnvalue) "Team B Won")
          (UserInterface|Viewport|AddtoViewport _returnvalue 0)
          (else
            (CallFunction|UpdateWidget :!label _label)))))
    (else
      (bind _result_2 (Math|Integer|DecrementInt (Variables|Default|GetNumberOfTeamB_Alive))
        (:%20%20
          (if (<= _result_2 0)
            (bind _returnvalue_2 (UserInterface|CreateWidget "/Game/WB_WinnerTeam.WB_WinnerTeam_C"))
            (Rendering|Components|TextRender|SetText (Variables|/Game/WB_WinnerTeam.WB_WinnerTeam_C|GetWinnerText _returnvalue_2) "Team A Won")
            (UserInterface|Viewport|AddtoViewport _returnvalue_2 0)
            (else
              (goto _label))))))))

(event Custom|Update%20Widget
  (bind _asbp_third_person_character (Utilities|Casting|CastToBP_ThirdPersonCharacter (Game|GetPlayerCharacter 0)))
  (Rendering|Components|TextRender|SetText (Variables|/Game/WB_HUD.WB_HUD_C|GetTeamAText (Variables|/Game/ThirdPerson/Blueprints/BP_ThirdPersonCharacter.BP_ThirdPersonCharacter_C|GetHUD _asbp_third_person_character)) (Utilities|Text|FormatText "Team A: {Value}" (Variables|Default|GetNumberOfTeamA_Alive)))
  (Rendering|Components|TextRender|SetText (Variables|/Game/WB_HUD.WB_HUD_C|GetTeamBText (Variables|/Game/ThirdPerson/Blueprints/BP_ThirdPersonCharacter.BP_ThirdPersonCharacter_C|GetHUD _asbp_third_person_character)) (Utilities|Text|FormatText "Team B: {Value}" (Variables|Default|GetNumberOfTeamB_Alive))))

(event EventBeginPlay
  (Utilities|FlowControl|Delay 0.4)
  (CallFunction|UpdateWidget))

(fn ConstructionScript)